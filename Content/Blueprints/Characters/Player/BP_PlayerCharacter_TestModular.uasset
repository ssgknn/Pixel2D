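; Test player character Blueprint that manages the inventory and notification UI.
; IA_Inventory flip-flops the inventory widget on and off screen, creating it on first use, while two input-mode nodes sit unconnected.
; A notification stack widget is created on BeginPlay, restored by ShowinGameUI for the locally controlled player after clearing all widgets, and fed messages through ShowNotificationBP.
; The X key sends a test message through ClientShowNotification, and debug prints trace the notification flow.
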(event `Key|X`
  (params (Key :type "Key Structure"))
  ;[1 1 1] teszt
  (:`Pressed`
    (`self.ClientShowNotification` "Test notification")))

(event `self.ReceiveBeginPlay`
  (`self.CreateNotofication UI`))

(event `EnhancedInput|/Game/Input/Actions/IA_Inventory`
  (params (ActionValue :type Boolean) (ElapsedSeconds :type "Float (double-precision)") (TriggeredSeconds :type "Float (double-precision)") (InputAction :type "InputAction Object Reference" :default "/Game/Input/Actions/IA_Inventory.IA_Inventory"))
  (bind _inventorywidget (`self.InventoryWidget`))
  (:`Started`
    (`/Engine/EditorBlueprintResources/StandardMacros.FlipFlop`
      (:`A`
        (`/Engine/EditorBlueprintResources/StandardMacros.IsValid` _inventorywidget
          (:`Is Valid`
            _)
          (:`Is Not Valid`
            (bind _returnvalue (`|CreateWidget` "/Game/Blueprints/UserInterface/WBP_Inventroy.WBP_Inventroy_C"))
            (set `self.InventoryWidget` _returnvalue)))
        (`UserWidget.AddToViewport` (`self.InventoryWidget`) 0))
      (:`B`
        (`Widget.RemoveFromParent` _inventorywidget)))))

(event `CreateNotofication UI`
  (`/Engine/EditorBlueprintResources/StandardMacros.IsValid` (`self.NotificationWidget`)
    (:`Is Valid`
      (`UserWidget.AddToViewport` (`self.NotificationWidget`) 0)
      (`KismetSystemLibrary.PrintString` "valid"))
    (:`Is Not Valid`
      (bind _returnvalue (`|CreateWidget` "/Game/Blueprints/UserInterface/WBP_NotificationStack.WBP_NotificationStack_C"))
      (bind _output_get (set `self.NotificationWidget` _returnvalue))
      (`UserWidget.AddToViewport` _output_get 0)
      (`KismetSystemLibrary.PrintString` "in_valid"))))

(event `self.ShowInGameUI`
  (if (`self.IsLocallyControlled`)
    (`WidgetLayoutLibrary.RemoveAllWidgets`)
    (`self.CreateNotofication UI`)
    (`KismetSystemLibrary.PrintString` "ingameUI")))

(event `self.ShowNotification_BP`
  (params (Message :type "Text (by ref)"))
  (bind _notificationwidget (`self.NotificationWidget`))
  (`/Engine/EditorBlueprintResources/StandardMacros.IsValid` _notificationwidget
    (:`Is Valid`
      (`/Game/Blueprints/UserInterface/WBP_NotificationStack.Add Notification` _notificationwidget Message)
      (`KismetSystemLibrary.PrintString` "Notifi"))))

(fn `UserConstructionScript`)