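; Player character Blueprint that manages the player's on-screen UI: main widget, inventory and notification stack.
; BeginPlay sets up the notification and main widgets, and the inventory input toggles a lazily created inventory widget via FlipFlop.
; UI events rebuild the notification layer for the locally controlled player and forward messages to the stack.
; Debug keys send a test notification, open MainWorld as a listen server, or call DEBUGKey.
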(event `Key|X`
  (params (Key :type "Key Structure"))
  ;[1 1 1] DEBUG
  (:`Pressed`
    (`self.ClientShowNotification` "Test notification")))

(event `Key|H`
  (params (Key :type "Key Structure"))
  ;[1 1 1] DEBUG
  (:`Pressed`
    (`KismetSystemLibrary.ExecuteConsoleCommand` "open MainWorld?listen" null)))

(event `Key|K`
  (params (Key :type "Key Structure"))
  ;[1 1 1] DEBUG
  (:`Pressed`
    (`KismetSystemLibrary.PrintString` "K_Debug")
    (`self.DEBUG_Key`)))

(event `self.ReceiveBeginPlay`
  ;[1 1 1] BeginPlay
  (`self.CreateNotofication UI`)
  (bind _returnvalue (`|GenericCreateObject` "/Game/Blueprints/UserInterface/WBP_Main.WBP_Main_C"))
  (`UserWidget.AddToViewport` _returnvalue 0))

(event `EnhancedInput|/Game/Input/Actions/IA_Inventory`
  (params (ActionValue :type Boolean) (ElapsedSeconds :type "Float (double-precision)") (TriggeredSeconds :type "Float (double-precision)") (InputAction :type "InputAction Object Reference" :default "/Game/Input/Actions/IA_Inventory.IA_Inventory"))
  (bind _inventorywidget (`self.InventoryWidget`))
  ;[1 1 1] Open/Close inventory
  (:`Started`
    (`/Engine/EditorBlueprintResources/StandardMacros.FlipFlop`
      (:`A`
        (`/Engine/EditorBlueprintResources/StandardMacros.IsValid` _inventorywidget
          (:`Is Valid`
            _)
          (:`Is Not Valid`
            (bind _returnvalue (`|CreateWidget` "/Game/Blueprints/UserInterface/Inventory/WBP_Inventroy.WBP_Inventroy_C"))
            (set `self.InventoryWidget` _returnvalue)))
        (`UserWidget.AddToViewport` (`self.InventoryWidget`) 0))
      (:`B`
        (`Widget.RemoveFromParent` _inventorywidget)))))

(event `CreateNotofication UI`
  (`/Engine/EditorBlueprintResources/StandardMacros.IsValid` (`self.NotificationWidget`)
    (:`Is Valid`
      (`UserWidget.AddToViewport` (`self.NotificationWidget`) 0)
      (`KismetSystemLibrary.PrintString` "valid"))
    (:`Is Not Valid`
      (bind _returnvalue (`|CreateWidget` "/Game/Blueprints/UserInterface/Notification/WBP_NotificationStack.WBP_NotificationStack_C"))
      (bind _output_get (set `self.NotificationWidget` _returnvalue))
      (`UserWidget.AddToViewport` _output_get 0)
      (`KismetSystemLibrary.PrintString` "in_valid"))))

(event `ShowInGameUI_1`
  (if (`self.IsLocallyControlled`)
    (`WidgetLayoutLibrary.RemoveAllWidgets`)
    (`self.CreateNotofication UI`)
    (`KismetSystemLibrary.PrintString` "ingameUI")))

(event `ShowNotification_BP_1`
  (params (Message :type "Text (by ref)"))
  (bind _notificationwidget (`self.NotificationWidget`))
  (`/Engine/EditorBlueprintResources/StandardMacros.IsValid` _notificationwidget
    (:`Is Valid`
      (`/Game/Blueprints/UserInterface/Notification/WBP_NotificationStack.Add Notification` _notificationwidget Message)
      (`KismetSystemLibrary.PrintString` "Notifi"))))

(fn `UserConstructionScript`)