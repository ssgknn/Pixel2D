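; BP_WorldHandler is a world handler Blueprint whose graph holds only disconnected startup logic for loading a named world.
; BeginPlay and the construction script are empty, so none of that logic runs.
; The unused chains, under an authority check, load player 0's WorldName into either a spawned handler or itself, then initialize that player's chunk variables and enable its tick.
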(event `self.ReceiveBeginPlay`)

(fn `UserConstructionScript`)